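; BP_Grave is a grave actor that is replaced by a new BP_AICharacter when triggered.
; On BeginPlay it registers itself with the BP_AIController of every existing AI character through AddGrave.
; SpawnCharacter spawns a character at the mesh, calls DelGrave on those controllers, then destroys the grave.
; DestroyGrave instead spawns at a random point in a box sized by mesh scale and self-destructs without deregistering.
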(event Custom|DestroyGrave
  (bind _staticmesh (Variables|Default|GetStaticMesh))
  (Game|SpawnActorfromClass "/Game/MyContent/BP_AICharacter.BP_AICharacter_C" (Math|Transform|MakeTransform (Math|Random|RandomPointinBoundingBox (Transformation|GetWorldLocation _staticmesh) (Transformation|GetWorldScale _staticmesh))) "AlwaysSpawn" 0 0)
  (Actor|DestroyActor))

(event EventBeginPlay
  (|CallParentFunction)
  (bind _outactors (Actor|GetAllActorsOfClass "/Game/MyContent/BP_AICharacter.BP_AICharacter_C"))
  (for _array_element _outactors
    (bind _asbp_aicontroller (Utilities|Casting|CastToBP_AIController (AI|GetAIController _array_element)))
    (Default|AddGrave _asbp_aicontroller self)))

(fn ConstructionScript)

(fn SpawnCharacter
  (Game|SpawnActorfromClass "/Game/MyContent/BP_AICharacter.BP_AICharacter_C" (Math|Transform|MakeTransform (Transformation|GetWorldLocation (Variables|Default|GetStaticMesh))) "Undefined" 0 0)
  (bind _outactors (Actor|GetAllActorsOfClass "/Game/MyContent/BP_AICharacter.BP_AICharacter_C"))
  (for _array_element _outactors
    (bind _asbp_aicontroller (Utilities|Casting|CastToBP_AIController (AI|GetAIController _array_element)))
    (Default|DelGrave _asbp_aicontroller self))
  (Actor|DestroyActor))