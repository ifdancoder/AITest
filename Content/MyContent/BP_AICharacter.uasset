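; BP_AICharacter is an AI-driven character that picks up crucifixion actors and leaves a grave when destroyed.
; Its interaction sphere, sized from InteractionRadius at BeginPlay, destroys any overlapping BP_Crucifixion and then calls AddCrucifixion on its BP_AIController.
; DestroyAICharacter spawns BP_Grave at the mesh location with default rotation and scale before removing the character.
; UpdateSpeed sets the movement component's maximum walk speed.
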(event OnComponentBeginOverlap(Sphere)
  (params (OverlappedComponent :type Primitive%20Component%20Object%20Reference) (OtherActor :type Actor%20Object%20Reference) (OtherComp :type Primitive%20Component%20Object%20Reference) (OtherBodyIndex :type Integer) (bFromSweep :type Boolean) (SweepResult :type Hit%20Result%20Structure%20%28by%20ref%29))
  (bind _asbp_crucifixion (Utilities|Casting|CastToBP_Crucifixion OtherActor))
  (Actor|DestroyActor _asbp_crucifixion)
  (bind _asbp_aicontroller (Utilities|Casting|CastToBP_AIController (Pawn|GetController)))
  (Default|AddCrucifixion _asbp_aicontroller))

(event Custom|DestroyAICharacter
  (Game|SpawnActorfromClass "/Game/MyContent/BP_Grave.BP_Grave_C" (Math|Transform|MakeTransform (Transformation|GetWorldLocation (Variables|Character|GetMesh))) "Undefined" 0 0)
  (Actor|DestroyActor))

(event EventBeginPlay
  (Components|Sphere|SetSphereRadius (Variables|Default|GetSphere) (Variables|Default|GetInteractionRadius) true))

(fn ConstructionScript)

(fn UpdateSpeed
  (params (NewSpeed :type Float%20%28single-precision%29))
  (Variables|/Script/Engine.CharacterMovementComponent|SetMaxWalkSpeed (Variables|Character|GetCharacterMovement) NewSpeed))